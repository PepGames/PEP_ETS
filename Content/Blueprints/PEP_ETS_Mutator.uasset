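; Mutator for the ETS mod that bootstraps its core systems onto player bipeds as they spawn.
; On each spawn notification for a Biped_Player, it adds the gameplay mod component if absent, then the save manager component, printing an on-screen confirmation for each.
; The save manager check runs only after the core is newly added, and SetReferences then cross-links the two components so each can reach the other.
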(event EventBeginPlay)

(event EventTick
  (params (DeltaSeconds :type Float%20%28single-precision%29)))

(event EventActorSpawnedNotification
  (params (SpawnedActor :type Actor%20Object%20Reference))
  (bind _output_get (Variables|Default|SetSpawnedActor SpawnedActor))
  ;[0.31 0 0] Check if component has already been added, and if not, we then add it to apply gameplay changing logic. LOAD MOD CORE
  (bind _asbiped_player (Utilities|Casting|CastToBiped_Player _output_get))
  (Utilities|IsValid (Actor|GetComponentbyClass _asbiped_player "/PEP_ETS/Blueprints/PEP_ETS_GameplayMod1.PEP_ETS_GameplayMod1_C")
    (:Is%20Not%20Valid
      (bind _returnvalue (Game|AddComponentbyClass _asbiped_player "/PEP_ETS/Blueprints/PEP_ETS_GameplayMod1.PEP_ETS_GameplayMod1_C"))
      (Variables|Default|SetPEP%20ETS%20GameplayMod _returnvalue)
      (Development|PrintString "ETS MOD CORE LOADED" true true "(R=1.000000,G=0.902413,B=0.000000,A=1.000000)" 2e+01)
      ;[0.31 0 0] Check if component has already been added, and if not, we then add it to apply gameplay changing logic. LOAD SAVE MANAGER
      (bind _asbiped_player_2 (Utilities|Casting|CastToBiped_Player (Variables|Default|GetSpawnedActor)))
      (Utilities|IsValid (Actor|GetComponentbyClass _asbiped_player_2 "/PEP_ETS/Blueprints/PEP_ETS_SaveManager.PEP_ETS_SaveManager_C")
        (:Is%20Not%20Valid
          (bind _returnvalue_2 (Game|AddComponentbyClass _asbiped_player_2 "/PEP_ETS/Blueprints/PEP_ETS_SaveManager.PEP_ETS_SaveManager_C"))
          (Variables|Default|SetPEP%20ETS%20SaveManager _returnvalue_2)
          (Development|PrintString "ETS SAVE MANAGER LOADED" true true "(R=1.000000,G=0.902413,B=0.000000,A=1.000000)" 2e+01)
          (CallFunction|SetReferences))))))

(fn SetReferences
  (Variables|/PEP_ETS/Blueprints/PEP_ETS_GameplayMod1.PEP_ETS_GameplayMod1_C|SetPEP%20ETS%20SaveManager (Variables|Default|GetPEP%20ETS%20GameplayMod) (Variables|Default|GetPEP%20ETS%20SaveManager))
  (Variables|/PEP_ETS/Blueprints/PEP_ETS_SaveManager.PEP_ETS_SaveManager_C|SetPEP%20ETS%20GameplayMod (Variables|Default|GetPEP%20ETS%20SaveManager) (Variables|Default|GetPEP%20ETS%20GameplayMod)))