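; Input actor for the PEP ETS talent-point mod that maps Shift+T to toggle its menu.
; Opening creates the core widget, disables player movement and binds its Apply, Remove and Unlock buttons to confirmation screens.
; Confirmed screens save the player level map and update points, remove points, or unlock them, then show a notification.
; The Apply screen previews retroactive and not-yet-earned points from per-level bonuses.
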(event Custom|ApplyScreenOpenedEvent
  ;[1 1 1] Bind to dispatcher for ApplyScreen
  (if (not (Variables|Default|GetIsApplyScreenOpen))
    (CallFunction|OpenApplyScreen)
    (EventDispatchers|BindEventtoPEPETSApplyScreenClosed (Variables|Default|GetPEP%20ETS%20ApplyScreen) (delegate Custom|ApplyScreenClosedEvent))))

(event Custom|ETSMenuClosed
  ;[1 1 1] Open/Close ETS Menu
  (if (Variables|Default|GetIsETSMenuOpen)
    (CallFunction|CloseAllScreens)
    (else
      (CallFunction|OpenETSMenu)
      (Utilities|FlowControl|Sequence
        (:then_0
          ;[1 1 1] Bind to dispatcher for ETSMenuClosed
          (EventDispatchers|BindEventtoETSMenuClosed (Variables|Default|GetPEP%20ETS%20WidgetCore) (delegate Custom|ETSMenuClosedEvent)))
        (:then_1
          ;[1 1 1] Bind to dispatcher for ApplyScreen
          (EventDispatchers|BindEventtoApplyButtonPressedEvent (Variables|Default|GetPEP%20ETS%20WidgetCore) (delegate Custom|ApplyScreenOpenedEvent)))
        (:then_2
          ;[1 1 1] Bind to dispatcher for RemoveScreen
          (EventDispatchers|BindEventtoRemoveButtonPressedEvent (Variables|Default|GetPEP%20ETS%20WidgetCore) (delegate Custom|RemoveScreenOpenedEvent)))
        (:then_3
          ;[1 1 1] Bind to dispatcher for UnlockScreen
          (EventDispatchers|BindEventtoUnlockButtonPressedEvent (Variables|Default|GetPEP%20ETS%20WidgetCore) (delegate Custom|UnlockScreenOpenedEvent)))))))

(event Custom|UnlockScreenClosedEvent
  (params (isApplyTrue :type Boolean))
  ;[1 1 1] Bind to dispatcher for UnlockScreen
  (CallFunction|UnlockScreenClosed isApplyTrue))

(event Custom|ApplyScreenClosedEvent
  (params (isApplyTrue :type Boolean))
  ;[1 1 1] Bind to dispatcher for ApplyScreen
  (CallFunction|ApplyScreenClosed isApplyTrue))

(event Custom|ApplyScreenClosed
  (params (IsApplyTrue :type Boolean))
  (bind _pep_ets_widgetcore (Variables|Default|GetPEP%20ETS%20WidgetCore))
  (bind _pep_ets_gameplaymod (Variables|/PEP_ETS/Blueprints/PEP_ETS_WidgetCore.PEP_ETS_WidgetCore_C|GetPEP%20ETS%20GameplayMod _pep_ets_widgetcore))
  ;[1 1 1] ApplyScreen is Closed
  (if IsApplyTrue
    (Default|UpdatePlayerLevelMapLive (Variables|/PEP_ETS/Blueprints/PEP_ETS_WidgetCore.PEP_ETS_WidgetCore_C|GetPEP%20ETS%20GameplayMod (Variables|Default|GetPEP%20ETS%20WidgetCore)))
    (Default|SavePlayerLevelMap _pep_ets_widgetcore)
    (Default|UpdateTalentPoints _pep_ets_gameplaymod)
    (bind _aspep_ets_save_manager (Utilities|Casting|CastToPEP_ETS_SaveManager (Variables|/PEP_ETS/Blueprints/PEP_ETS_GameplayMod1.PEP_ETS_GameplayMod1_C|GetPEP%20ETS%20SaveManager _pep_ets_gameplaymod)))
    (Default|SaveETSMisc _aspep_ets_save_manager)
    (CallFunction|CloseApplyScreen)
    (CallFunction|CreateTalentNotification)
    (else
      (CallFunction|CloseApplyScreen))))

(event Custom|ETSMenuClosedEvent
  ;[1 1 1] Bind to dispatcher for ETSMenuClosed
  (CallFunction|ETSMenuClosed))

(event Custom|RemoveScreenOpenedEvent
  ;[1 1 1] Bind to dispatcher for RemoveScreen
  (if (not (Variables|Default|GetIsRemoveScreenOpen))
    (CallFunction|OpenRemoveScreen)
    (EventDispatchers|BindEventtoPEPETSRemoveScreenClosed (Variables|Default|GetPEP%20ETS%20RemoveScreen) (delegate Custom|RemoveScreenClosedEvent))))

(event Custom|RemoveScreenClosedEvent
  (params (IsRemoveTrue :type Boolean))
  ;[1 1 1] Bind to dispatcher for RemoveScreen
  (CallFunction|RemoveScreenClosed IsRemoveTrue))

(event Custom|RemoveScreenClosed
  (params (IsRemoveTrue :type Boolean))
  ;[1 1 1] RemoveScreen is Closed
  (if IsRemoveTrue
    (CallFunction|RemoveTalentPoints)
    (CallFunction|CloseRemoveScreen)
    (CallFunction|CreateTalentNotification)
    (else
      (CallFunction|CloseRemoveScreen))))

(event Custom|UnlockScreenOpenedEvent
  ;[1 1 1] Bind to dispatcher for UnlockScreen
  (if (not (Variables|Default|GetIsUnlockScreenOpen))
    (CallFunction|OpenUnlockScreen)
    (EventDispatchers|BindEventtoPEPETSUnlockScreenClosed (Variables|Default|GetPEP%20ETS%20UnlockScreen) (delegate Custom|UnlockScreenClosedEvent))))

(event Custom|UnlockScreenClosed
  (params (IsUnlockTrue :type Boolean))
  ;[1 1 1] UnlockScreen is Closed
  (if IsUnlockTrue
    (CallFunction|UnlockTalentPoints)
    (CallFunction|CloseUnlockScreen)
    (CallFunction|CreateTalentNotification)
    (else
      (CallFunction|CloseUnlockScreen))))

(event EventBeginPlay
  (Utilities|FlowControl|Sequence
    (:then_0
      (Utilities|SetTKey))))

(event Input|ActionEvents|InputActionLevelup
  (params (Key :type Key%20Structure :default "None"))
  ;[1 1 1] Debug RaisePlayerLevelByOne cheat
)

(event Input|ActionEvents|InputActionToggleETSMenu
  (params (Key :type Key%20Structure :default "None"))
  ;[1 1 1] Open/Close ETS Menu
  (:Pressed
    (if (Variables|Default|GetIsETSMenuOpen)
      (CallFunction|CloseAllScreens)
      (else
        (CallFunction|OpenETSMenu)
        (Utilities|FlowControl|Sequence
          (:then_0
            ;[1 1 1] Bind to dispatcher for ETSMenuClosed
            (EventDispatchers|BindEventtoETSMenuClosed (Variables|Default|GetPEP%20ETS%20WidgetCore) (delegate Custom|ETSMenuClosedEvent)))
          (:then_1
            ;[1 1 1] Bind to dispatcher for ApplyScreen
            (EventDispatchers|BindEventtoApplyButtonPressedEvent (Variables|Default|GetPEP%20ETS%20WidgetCore) (delegate Custom|ApplyScreenOpenedEvent)))
          (:then_2
            ;[1 1 1] Bind to dispatcher for RemoveScreen
            (EventDispatchers|BindEventtoRemoveButtonPressedEvent (Variables|Default|GetPEP%20ETS%20WidgetCore) (delegate Custom|RemoveScreenOpenedEvent)))
          (:then_3
            ;[1 1 1] Bind to dispatcher for UnlockScreen
            (EventDispatchers|BindEventtoUnlockButtonPressedEvent (Variables|Default|GetPEP%20ETS%20WidgetCore) (delegate Custom|UnlockScreenOpenedEvent))))))))

(fn ConstructionScript)

(fn OpenETSMenu
  (bind _returnvalue (Game|GetPlayerController 0))
  (Pawn|Components|CharacterMovement|DisableMovement (Variables|/Script/Engine.Character|GetCharacterMovement (Class|BipedPlayer|GettheBipedPlayer)))
  (bind _returnvalue_2 (UserInterface|CreateWidget "/PEP_ETS/Blueprints/PEP_ETS_WidgetCore.PEP_ETS_WidgetCore_C" _returnvalue))
  (bind _output_get (Variables|Default|SetPEP%20ETS%20WidgetCore _returnvalue_2))
  (UserInterface|Viewport|AddtoViewport _output_get 0)
  (Input|SetInputModeUIOnly _returnvalue _output_get "DoNotLock")
  (Class|UIManager|ShowVirtualCursor (Class|UIManager|GetUIManagerPure) _returnvalue true "(X=0.500000,Y=0.500000)" "None")
  (Variables|Default|SetIsETSMenuOpen true))

(fn CloseETSMenu
  (bind _returnvalue (Game|GetPlayerController 0))
  (bind _pep_ets_widgetcore (Variables|Default|GetPEP%20ETS%20WidgetCore))
  (if (Variables|Default|GetIsETSMenuOpen)
    (EventDispatchers|UnbindallEventsfromApplyButtonPressedEvent _pep_ets_widgetcore)
    (EventDispatchers|UnbindallEventsfromRemoveButtonPressedEvent _pep_ets_widgetcore)
    (EventDispatchers|UnbindallEventsfromETSMenuClosed _pep_ets_widgetcore)
    (Widget|RemovefromParent _pep_ets_widgetcore)
    (Input|SetInputModeGameOnly _returnvalue)
    (Class|UIManager|ShowVirtualCursor (Class|UIManager|GetUIManagerPure) _returnvalue false "(X=0.500000,Y=0.500000)" "None")
    (Variables|Default|SetIsETSMenuOpen false)
    (Pawn|Components|CharacterMovement|SetMovementMode (Variables|/Script/Engine.Character|GetCharacterMovement (Class|BipedPlayer|GettheBipedPlayer)) "MOVE_Walking" 0)
    (return)
    (else
      (return))))

(fn OpenApplyScreen
  (bind _returnvalue (UserInterface|CreateWidget "/PEP_ETS/Blueprints/PEP_ETS_ApplyScreen.PEP_ETS_ApplyScreen_C" (Game|GetPlayerController 0)))
  (bind _output_get (Variables|Default|SetPEP%20ETS%20ApplyScreen _returnvalue))
  (CallFunction|SetApplyScreenDynamicText _output_get)
  (UserInterface|Viewport|AddtoViewport _output_get 0)
  (Widget|SetFocus _output_get)
  (Variables|Default|SetIsApplyScreenOpen true))

(fn CloseApplyScreen
  (bind _pep_ets_applyscreen (Variables|Default|GetPEP%20ETS%20ApplyScreen))
  (if (Variables|Default|GetIsApplyScreenOpen)
    (EventDispatchers|UnbindallEventsfromPEPETSApplyScreenClosed _pep_ets_applyscreen)
    (Widget|RemovefromParent _pep_ets_applyscreen)
    (Widget|SetFocus (Variables|Default|GetPEP%20ETS%20WidgetCore))
    (Variables|Default|SetIsApplyScreenOpen false)
    (return)
    (else
      (return))))

(fn OpenRemoveScreen
  (bind _returnvalue (UserInterface|CreateWidget "/PEP_ETS/Blueprints/PEP_ETS_RemoveScreen.PEP_ETS_RemoveScreen_C" (Game|GetPlayerController 0)))
  (bind _output_get (Variables|Default|SetPEP%20ETS%20RemoveScreen _returnvalue))
  (CallFunction|SetRemoveScreenDynamicText _output_get)
  (UserInterface|Viewport|AddtoViewport _output_get 0)
  (Widget|SetFocus _output_get)
  (Variables|Default|SetIsRemoveScreenOpen true))

(fn CloseRemoveScreen
  (bind _pep_ets_removescreen (Variables|Default|GetPEP%20ETS%20RemoveScreen))
  (if (Variables|Default|GetIsRemoveScreenOpen)
    (EventDispatchers|UnbindallEventsfromPEPETSRemoveScreenClosed _pep_ets_removescreen)
    (Widget|RemovefromParent _pep_ets_removescreen)
    (Widget|SetFocus (Variables|Default|GetPEP%20ETS%20WidgetCore))
    (Variables|Default|SetIsRemoveScreenOpen false)
    (return)
    (else
      (return))))

(fn GetUnrealizedTalentPoints
  (params (PlayerLevelMapLive :type Map%20of%20Integers%20to%20Integers))
  (bind _extra_not_earned_by_now (CallFunction|GetExtraNotEarnedbyNow PlayerLevelMapLive))
  (return (Utilities|Text|ToText(Integer) _extra_not_earned_by_now)))

(fn GetRetroactiveTalentPoints
  (params (PlayerLevelMapLive :type Map%20of%20Integers%20to%20Integers))
  (bind _extra_earned_by_now (CallFunction|GetExtraEarnedbyNow PlayerLevelMapLive))
  (LocalVariables|SetExtraEarnedByNow _extra_earned_by_now)
  (bind _vanillatalentpoints (Default|GetVanillaTalentPoints (Variables|/PEP_ETS/Blueprints/PEP_ETS_WidgetCore.PEP_ETS_WidgetCore_C|GetPEP%20ETS%20GameplayMod (Variables|Default|GetPEP%20ETS%20WidgetCore))))
  (LocalVariables|SetDesiredTotalOwnedNow (+ _vanillatalentpoints (LocalVariables|GetExtraEarnedByNow)))
  (bind _totalperksinuse (CallFunction|GetTotalPerksinUse))
  (return (Utilities|Text|ToText(Integer) (Math|Integer|Clamp(Integer) (- (LocalVariables|GetDesiredTotalOwnedNow) _totalperksinuse) 0 123456789))))

(fn GetExtraEarnedbyNow
  (params (PlayerLevelMap :type Map%20of%20Integers%20to%20Integers))
  ;[1 1 1] Clear Local Variable
  (LocalVariables|SetExtraEarnedByNow 0)
  ;[1 1 1] ForEach entry in the PlayerLevelMap find how many ExtraPoints they should have and return the total
  (for _index (range 1 (Variables|/PEP_ETS/Blueprints/PEP_ETS_GameplayMod1.PEP_ETS_GameplayMod1_C|GetCurrentPlayerLevel (Variables|/PEP_ETS/Blueprints/PEP_ETS_WidgetCore.PEP_ETS_WidgetCore_C|GetPEP%20ETS%20GameplayMod (Variables|Default|GetPEP%20ETS%20WidgetCore))))
    (LocalVariables|SetExtraEarnedByNow (+ (LocalVariables|GetExtraEarnedByNow) (.Value (Utilities|Map|Find PlayerLevelMap _index)))))
  (return (LocalVariables|GetExtraEarnedByNow)))

(fn GetExtraNotEarnedbyNow
  (params (PlayerLevelMap :type Map%20of%20Integers%20to%20Integers))
  ;[1 1 1] Clear Local Variable
  (LocalVariables|SetExtraNotEarnedByNow 0)
  ;[1 1 1] ForEach entry in the PlayerLevelMap find how many ExtraPoints they haven't reached the level for and return the total
  (for _index (range (+ (Variables|/PEP_ETS/Blueprints/PEP_ETS_GameplayMod1.PEP_ETS_GameplayMod1_C|GetCurrentPlayerLevel (Variables|/PEP_ETS/Blueprints/PEP_ETS_WidgetCore.PEP_ETS_WidgetCore_C|GetPEP%20ETS%20GameplayMod (Variables|Default|GetPEP%20ETS%20WidgetCore))) 1) (Utilities|Map|Length PlayerLevelMap))
    (LocalVariables|SetExtraNotEarnedByNow (+ (LocalVariables|GetExtraNotEarnedByNow) (.Value (Utilities|Map|Find PlayerLevelMap _index)))))
  (return (LocalVariables|GetExtraNotEarnedByNow)))

(fn SetApplyScreenDynamicText
  (params (ApplyScreen :type PEP%20ETS%20Apply%20Screen%20Object%20Reference))
  ;[1 1 1] Set local refs and Update PlayerLevelMapLive with most recent stored data from the User's Inputs
  (LocalVariables|SetApplyScreenRef ApplyScreen)
  (bind _playerlevelmaplive (Default|UpdatePlayerLevelMapLive (Variables|/PEP_ETS/Blueprints/PEP_ETS_WidgetCore.PEP_ETS_WidgetCore_C|GetPEP%20ETS%20GameplayMod (Variables|Default|GetPEP%20ETS%20WidgetCore))))
  (LocalVariables|SetPlayerLevelMapLive _playerlevelmaplive)
  (Utilities|FlowControl|Sequence
    (:then_0
      ;[1 1 1] SetText for projected RetroactiveTalentPoints
      (bind _newretroactivepointsamount (CallFunction|GetRetroactiveTalentPoints (LocalVariables|GetPlayerLevelMapLive)))
      (Rendering|Components|TextRender|SetText (Variables|/PEP_ETS/Blueprints/PEP_ETS_ApplyScreen.PEP_ETS_ApplyScreen_C|GetNewRetroactivePointsAmount (LocalVariables|GetApplyScreenRef)) _newretroactivepointsamount))
    (:then_1
      ;[1 1 1] SetText for projected UnrealizedTalentPoints
      (bind _newunrealizedpointsamount (CallFunction|GetUnrealizedTalentPoints (LocalVariables|GetPlayerLevelMapLive)))
      (Rendering|Components|TextRender|SetText (Variables|/PEP_ETS/Blueprints/PEP_ETS_ApplyScreen.PEP_ETS_ApplyScreen_C|GetNewUnrealizedPointsAmount (LocalVariables|GetApplyScreenRef)) _newunrealizedpointsamount))
    (:then_2
      (return))))

(fn SetRemoveScreenDynamicText
  (params (RemoveScreen :type PEP%20ETS%20Remove%20Screen%20Object%20Reference))
  ;[1 1 1] Set local ref
  (LocalVariables|SetRemoveScreenRef RemoveScreen)
  (Utilities|FlowControl|Sequence
    (:then_0
      ;[1 1 1] SetText for CurrentAvailablePoints
      (bind _returnvalue (Class|PerksTree|GetPerkPoints))
      (Rendering|Components|TextRender|SetText (Variables|/PEP_ETS/Blueprints/PEP_ETS_RemoveScreen.PEP_ETS_RemoveScreen_C|GetCurrentAvailablePointsValue (LocalVariables|GetRemoveScreenRef)) (Utilities|Text|ToText(Integer) _returnvalue)))
    (:then_1
      ;[1 1 1] SetText for CurrentlyInvestedTalents
      (Rendering|Components|TextRender|SetText (Variables|/PEP_ETS/Blueprints/PEP_ETS_RemoveScreen.PEP_ETS_RemoveScreen_C|GetInvestedTalentsValue (LocalVariables|GetRemoveScreenRef)) (Utilities|Text|ToText(Integer) (Class|PerksTree|GetPurchasedPerkCount "All"))))
    (:then_2
      ;[1 1 1] SetText for CurrentlyOwnedExtraPoints
      (bind _current_extra_points (Default|GetExtraTalentPoints (Variables|/PEP_ETS/Blueprints/PEP_ETS_WidgetCore.PEP_ETS_WidgetCore_C|GetPEP%20ETS%20GameplayMod (Variables|Default|GetPEP%20ETS%20WidgetCore))))
      (Rendering|Components|TextRender|SetText (Variables|/PEP_ETS/Blueprints/PEP_ETS_RemoveScreen.PEP_ETS_RemoveScreen_C|GetExtraPointsOwnedValue (LocalVariables|GetRemoveScreenRef)) (Utilities|Text|ToText(Integer) _current_extra_points)))
    (:then_3
      (return))))

(fn CreateTalentNotification
  (bind _returnvalue (UserInterface|CreateWidget "/PEP_ETS/Blueprints/PEP_ETS_Notification.PEP_ETS_Notification_C" (Game|GetPlayerController 0)))
  (UserInterface|Viewport|AddtoViewport _returnvalue 0)
  (return _returnvalue))

(fn RemoveTalentPoints
  (LocalVariables|SetRemoveAmount (Math|Float|Round (Class|SpinBox|GetValue (Variables|/PEP_ETS/Blueprints/PEP_ETS_RemoveScreen.PEP_ETS_RemoveScreen_C|GetPointsToRemoveValue (Variables|Default|GetPEP%20ETS%20RemoveScreen)))))
  (bind _returnvalue (Class|PerksTree|GetPerkPoints))
  (LocalVariables|SetAvailableNowPool _returnvalue)
  (bind _vanillatalentpoints (Default|GetVanillaTalentPoints (Variables|/PEP_ETS/Blueprints/PEP_ETS_WidgetCore.PEP_ETS_WidgetCore_C|GetPEP%20ETS%20GameplayMod (Variables|Default|GetPEP%20ETS%20WidgetCore))))
  (LocalVariables|SetMinAvailable (Math|Integer|Max(Integer) (- _vanillatalentpoints (Class|PerksTree|GetPurchasedPerkCount "All"))))
  (CallFunction|SetPerkPoints (Math|Integer|Max(Integer) (Math|Integer|Max(Integer) (LocalVariables|GetMinAvailable) (- (LocalVariables|GetAvailableNowPool) (LocalVariables|GetRemoveAmount))))))

(fn OpenUnlockScreen
  (bind _returnvalue (UserInterface|CreateWidget "/PEP_ETS/Blueprints/PEP_ETS_UnlockScreen.PEP_ETS_UnlockScreen_C" (Game|GetPlayerController 0)))
  (bind _output_get (Variables|Default|SetPEP%20ETS%20UnlockScreen _returnvalue))
  (UserInterface|Viewport|AddtoViewport _output_get 0)
  (Widget|SetFocus _output_get)
  (Variables|Default|SetIsUnlockScreenOpen true))

(fn CloseUnlockScreen
  (bind _pep_ets_unlockscreen (Variables|Default|GetPEP%20ETS%20UnlockScreen))
  (if (Variables|Default|GetIsUnlockScreenOpen)
    (EventDispatchers|UnbindallEventsfromPEPETSUnlockScreenClosed _pep_ets_unlockscreen)
    (Widget|RemovefromParent _pep_ets_unlockscreen)
    (Widget|SetFocus (Variables|Default|GetPEP%20ETS%20WidgetCore))
    (Variables|Default|SetIsUnlockScreenOpen false)
    (return)
    (else
      (return))))

(fn CloseAllScreens
  (CallFunction|CloseApplyScreen)
  (CallFunction|CloseRemoveScreen)
  (CallFunction|CloseUnlockScreen)
  (CallFunction|CloseETSMenu))