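; Save manager for the PEP ETS gameplay mod that persists player level data in the misc save database.
; BeginPlay calls UserSaveGameData, and SaveETSMisc writes each of the mod's PlayerLevelMap entries as a string under a prefixed key.
; LoadETSMisc reads those keys back, falls back to the mod's current value for missing entries, rebuilds PEPETSStruct and broadcasts MiscDBLoadCompleted.
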(event EventBeginPlay
  (bind _returnvalue (Class|SaveManager|Get))
  (Class|SaveManager|UserSaveGameData _returnvalue))

(event EventTick
  (params (DeltaSeconds :type Float%20%28single-precision%29)))

(fn SaveETSMisc
  (bind _pep_ets_gameplaymod (Variables|Default|GetPEP%20ETS%20GameplayMod))
  (bind _pep_ets_struct (Variables|/PEP_ETS/Blueprints/PEP_ETS_GameplayMod1.PEP_ETS_GameplayMod1_C|GetPEP%20ETS%20Struct _pep_ets_gameplaymod))
  (bind _playerlevelmap (Utilities|Struct|BreakPEP_ETS_Struct _pep_ets_struct))
  (bind _keys (Utilities|Map|Keys _playerlevelmap))
  (for _array_element _keys
    (Class|DbGateway|DbWriteMiscSaveDataItem (LocalVariables|GetDefaultOwner) (Utilities|String|Append "PlayerLevel." (Utilities|String|ToString(Integer) _array_element)) (Utilities|String|ToString(Integer) (.Value (Utilities|Map|Find _playerlevelmap _array_element))) false)))

(fn LoadETSMisc
  (bind _keys (Utilities|Map|Keys (Utilities|Struct|BreakPEP_ETS_Struct (Variables|/PEP_ETS/Blueprints/PEP_ETS_GameplayMod1.PEP_ETS_GameplayMod1_C|GetPEP%20ETS%20Struct (Variables|Default|GetPEP%20ETS%20GameplayMod)))))
  (for _array_element _keys
    (LocalVariables|SetLoopKey _array_element)
    (LocalVariables|SetLoopDefaultValue (.Value (Utilities|Map|Find (Utilities|Struct|BreakPEP_ETS_Struct (Variables|/PEP_ETS/Blueprints/PEP_ETS_GameplayMod1.PEP_ETS_GameplayMod1_C|GetPEP%20ETS%20Struct (Variables|Default|GetPEP%20ETS%20GameplayMod))) _array_element)))
    (bind (_outvalue _returnvalue) (Class|DbGateway|DbReadMiscSaveDataItem (LocalVariables|GetDefaultOwner) (Utilities|String|Append "PlayerLevel." (Utilities|String|ToString(Integer) _array_element))))
    (if _returnvalue
      (Utilities|Map|Add (LocalVariables|GetPlayerLevelMap) (LocalVariables|GetLoopKey) (Math|Conversions|ToInteger(Byte) _outvalue))
      (else
        (Utilities|Map|Add (LocalVariables|GetPlayerLevelMap) (LocalVariables|GetLoopKey) (LocalVariables|GetLoopDefaultValue)))))
  (Variables|Default|SetPEP%20ETS%20Struct (Utilities|Struct|MakePEP_ETS_Struct (LocalVariables|GetPlayerLevelMap)))
  (Default|CallMiscDBLoadCompleted))