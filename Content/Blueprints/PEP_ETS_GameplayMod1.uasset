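; Gameplay mod core for PEP ETS that grants extra talent points by player experience level.
; On BeginPlay it loads the misc config through the SaveManager, attaches an input actor to the biped player, and binds to level changes.
; Each level change tops up perk points: vanilla points from level five plus the saved per-level map, minus perks in use, clamped at zero.
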(event Custom|LevelChangeCheck
  (params (ExpLevel :type Integer) (bIndicateHUD :type Boolean))
  ;[1 1 1] Set the player's current Experience Level in the Mod Core and Bind an event to update it on ExperienceLevelChange
  (Variables|Default|SetCurrentPlayerLevel ExpLevel)
  (CallFunction|UpdateTalentPoints)
  (Development|PrintString "Talents updated!" true true "(R=0.000000,G=0.660000,B=1.000000,A=1.000000)" 5.0))

(event Custom|MiscLoadCompleted
  ;[1 1 1] Init the SaveManager and Bind set reference on AsyncLoadCompleted
  (Variables|Default|SetPEP%20ETS%20Struct (Variables|/PEP_ETS/Blueprints/PEP_ETS_SaveManager.PEP_ETS_SaveManager_C|GetPEP%20ETS%20Struct (stale EventBeginPlay _aspep_ets_save_manager))))

(event EventBeginPlay
  ;[1 1 1] Init the SaveManager and Bind set reference on AsyncLoadCompleted
  (Utilities|InitSaveManager
    (:Completed
      (bind _aspep_ets_save_manager (Utilities|Casting|CastToPEP_ETS_SaveManager (Variables|Default|GetPEP%20ETS%20SaveManager)))
      (EventDispatchers|BindEventtoMiscDBLoadCompleted _aspep_ets_save_manager (delegate Custom|MiscLoadCompleted))
      ;[1 1 1] Attach InputActor
      (Utilities|AttachInputActortoBipedPlayer
        (:Completed
          ;[1 1 1] Set the player's current Experience Level in the Mod Core and Bind an event to update it on ExperienceLevelChange
          (bind _returnvalue (Class|ExperienceManager|Get))
          (CallFunction|InitPlayerLevel _returnvalue)
          (EventDispatchers|BindEventtoMonExperienceLevelChangedDelegate _returnvalue (delegate Custom|LevelChangeCheck)))))))

(event EventTick
  (params (DeltaSeconds :type Float%20%28single-precision%29))
  ;[0.31 0 0] Dont use this for complex logic.
  ; its expensive!!
)

(fn UpdateTalentPoints
  (CallFunction|GetTalentPointstoAdd)
  (CallFunction|GetVanillaTalentPoints)
  ;[1 1 1] How many talent points has the player ever possesed
  (bind _totalperksinuse (CallFunction|GetTotalPerksinUse))
  ;[1 1 1] Add (VanillaTalentPoints+TalentPointsToAdd) - (Total Talent Points Owned) to the players current Perk amount
  (Class|PerksTree|UpdatePerkPoints (Math|Integer|Clamp(Integer) (- (+ (Variables|Default|GetVanillaTalentPoints) (Variables|Default|GetTalentPointsToAdd)) _totalperksinuse) 0 123456789)))

(fn InitPlayerLevel
  (params (Experience%20Manger :type Experience%20Manager%20Object%20Reference))
  ;[1 1 1] Store a copy of the player's current experience level
  (bind _returnvalue (Class|ExperienceManager|GetExperienceLevel Experience%20Manger))
  (Variables|Default|SetCurrentPlayerLevel _returnvalue))

(fn UpdatePlayerLevelMapLive
  ;[1 1 1] Get all children of the VerticalBox and ForEach, Cast to RowWidget
  (for _array_element (Class|PanelWidget|GetAllChildren (Variables|/PEP_ETS/Blueprints/PEP_ETS_WidgetCore.PEP_ETS_WidgetCore_C|GetRowWidgetBox (Variables|/PEP_ETS/Blueprints/PEP_ETS_InputActor.PEP_ETS_InputActor_C|GetPEP%20ETS%20WidgetCore (Variables|Default|GetPEP%20ETS%20InputActor))))
    (bind _aspep_ets_row_widget (Utilities|Casting|CastToPEP_ETS_RowWidget _array_element))
    ;[1 1 1] Get the points the player chose and adds them to the PlayerLevelMapLive
    (bind (_key _value) (Default|GetAssignedPoints _aspep_ets_row_widget))
    (Utilities|Map|Add (Variables|/PEP_ETS/Blueprints/PEP_ETS_WidgetCore.PEP_ETS_WidgetCore_C|GetPlayerLevelMapLive (Variables|/PEP_ETS/Blueprints/PEP_ETS_InputActor.PEP_ETS_InputActor_C|GetPEP%20ETS%20WidgetCore (Variables|Default|GetPEP%20ETS%20InputActor))) _key _value))
  (return (Variables|/PEP_ETS/Blueprints/PEP_ETS_WidgetCore.PEP_ETS_WidgetCore_C|GetPlayerLevelMapLive (Variables|/PEP_ETS/Blueprints/PEP_ETS_InputActor.PEP_ETS_InputActor_C|GetPEP%20ETS%20WidgetCore (Variables|Default|GetPEP%20ETS%20InputActor)))))

(fn GetVanillaTalentPoints
  ;[1 1 1] Clear Variable
  (Variables|Default|SetVanillaTalentPoints 0)
  ;[1 1 1] ForEach level from 1-CurrentPlayerLevel, if it's greater than or equal to 5 add 1 to VanillaTalentPoints
  (for _index (range 1 (Variables|Default|GetCurrentPlayerLevel))
    (if (>= _index 5)
      (Variables|Default|SetVanillaTalentPoints (+ (Variables|Default|GetVanillaTalentPoints) 1))))
  (return (Variables|Default|GetVanillaTalentPoints)))

(fn GetTalentPointstoAdd
  (bind _pep_ets_struct (Variables|Default|GetPEP%20ETS%20Struct))
  (bind _playerlevelmap (Utilities|Struct|BreakPEP_ETS_Struct _pep_ets_struct))
  ;[1 1 1] Clear Variable
  (Variables|Default|SetTalentPointsToAdd 0)
  ;[1 1 1] Grab Level Keys
  (bind _keys (Utilities|Map|Keys _playerlevelmap))
  ;[1 1 1] ForEach Level Key, FIND the amount of points to add if they are less than or equal to the Player's Current Level
  (for _array_element _keys
    (if (<= _array_element (Variables|Default|GetCurrentPlayerLevel))
      (Variables|Default|SetTalentPointsToAdd (+ (Variables|Default|GetTalentPointsToAdd) (.Value (Utilities|Map|Find _playerlevelmap _array_element))))))
  (return (Variables|Default|GetTalentPointsToAdd)))

(fn GetExtraTalentPoints
  ;[1 1 1] Subtract how many VanillaPoints the player should have, by how many perks they own
  (bind _totalperksinuse (CallFunction|GetTotalPerksinUse))
  (bind _vanillatalentpoints (CallFunction|GetVanillaTalentPoints))
  (return (Math|Integer|Clamp(Integer) (- _totalperksinuse _vanillatalentpoints) 0 123456789)))